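; SplineMesh_BP is a spline actor from HB_SimpleStreets that deforms a chosen static mesh along its spline.
; The construction script adds a spline mesh per segment, with configurable forward axis and collision, fitted to the local point locations and tangents.
; FlipMesh reverses a segment by swapping endpoints and negating tangents, while AddFlipSide adds a second, reversed copy.
; The event graph is inactive, and the array and segment helper functions are never called here.
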(fn `AddRemoveSegments`
  (params (Value :type "Integer (by ref)"))
  (if false
    _
    (elif false
      _)))

(fn `AddSplineMeshComponents`
  (params (SegmentCount :type Integer) (TargetArray :type "Array of SplineMeshComponent Object Reference (by ref)") (Offset :type "Float (double-precision)") (Collision :type Boolean))
  (locals (Counter :type Integer) (ComponentArray :type "Array of SplineMeshComponent Object Reference") (TargetSegmentCount :type Integer))
  (set `local.TargetSegmentCount` SegmentCount)
  (`/Engine/EditorBlueprintResources/StandardMacros.IncrementInt` (`local.Counter`) :!label _label
    (:`  `
      (bind _returnvalue (`AddComponent|NODE_AddSplineMeshComponent-0`))
      (if Collision
        (`PrimitiveComponent.SetCollisionEnabled` _returnvalue "QueryAndPhysics"))
      (`KismetArrayLibrary.Array_Add` TargetArray _returnvalue)
      (`/Engine/EditorBlueprintResources/StandardMacros.CompareInt` (`local.TargetSegmentCount`) (`local.Counter`)
        (:`>`
          (goto _label))
        (:`==`
          (return))))))

(fn `ReplaceVectorArrayValues`
  (params (From :type "Array of Vector Structure") (To :type "Array of Vector Structure (by ref)"))
  (for (_array_element _array_index) From
    (`KismetArrayLibrary.Array_Set` To _array_index _array_element))
  (return))

(fn `ResetVectorArray`
  (params (Array1 :type "Array of Vector Structure (by ref)") (Array2 :type "Array of Vector Structure") (Array3 :type "Array of Vector Structure") (Size :type Integer))
  (`KismetArrayLibrary.Array_Clear` Array1)
  (`KismetArrayLibrary.Array_Resize` Array1 Size)
  (`KismetArrayLibrary.Array_Clear` Array2)
  (`KismetArrayLibrary.Array_Resize` Array2 Size)
  (`KismetArrayLibrary.Array_Clear` Array3)
  (`KismetArrayLibrary.Array_Resize` Array3 Size))

(fn `UserConstructionScript`
  (bind (_location _tangent) (`SplineComponent.GetLocationAndTangentAtSplinePoint` (`self.Spline`) (`self.SplinePoint`) "Local"))
  (bind (_location_2 _tangent_2) (`SplineComponent.GetLocationAndTangentAtSplinePoint` (`self.Spline`) (`self.SplinePoint`) "Local"))
  (bind (_location_3 _tangent_3) (`SplineComponent.GetLocationAndTangentAtSplinePoint` (`self.Spline`) (`self.SplinePoint`) "Local"))
  (bind (_location_4 _tangent_4) (`SplineComponent.GetLocationAndTangentAtSplinePoint` (`self.Spline`) (+ (`self.SplinePoint`) 1) "Local"))
  (bind (_location_5 _tangent_5) (`SplineComponent.GetLocationAndTangentAtSplinePoint` (`self.Spline`) (+ (`self.SplinePoint`) 1) "Local"))
  (bind (_location_6 _tangent_6) (`SplineComponent.GetLocationAndTangentAtSplinePoint` (`self.Spline`) (+ (`self.SplinePoint`) 1) "Local"))
  (for _index (range (+ (- (`SplineComponent.GetNumberOfSplinePoints` (`self.Spline`)) 2) 1))
    (set `self.SplinePoint` _index)
    (`|ExecutionSequence`
      (:`then_0`
        (bind _returnvalue (`AddComponent|NODE_AddSplineMeshComponent-1`))
        (bind _output_get (set `self.SplineMesh` _returnvalue))
        (`StaticMeshComponent.SetStaticMesh` _output_get (`self.StaticMesh`))
        (`SplineMeshComponent.SetForwardAxis` (`self.SplineMesh`) (`self.ForwardAxis`) true)
        (`PrimitiveComponent.SetCollisionEnabled` (`self.SplineMesh`) (`self.Collision`))
        (`SceneComponent.K2_AttachToComponent` (`self.SplineMesh`) null "None" "KeepRelative" "KeepRelative" "KeepRelative" true)
        (if (not (`self.FlipMesh`))
          (`SplineMeshComponent.SetStartAndEnd` (`self.SplineMesh`) _location _tangent _location_4 _tangent_4 true)
          (else
            (`SplineMeshComponent.SetStartAndEnd` (`self.SplineMesh`) _location_5 (* _tangent_5 -1.0) _location_2 (* _tangent_2 -1.0) true))))
      (:`then_1`
        (if (`self.AddFlipSide`)
          (bind _returnvalue_2 (`AddComponent|NODE_AddSplineMeshComponent-2`))
          (bind _output_get_2 (set `self.SplineMesh2` _returnvalue_2))
          (`StaticMeshComponent.SetStaticMesh` _output_get_2 (`self.StaticMesh`))
          (`SplineMeshComponent.SetForwardAxis` (`self.SplineMesh2`) (`self.ForwardAxis`) true)
          (`PrimitiveComponent.SetCollisionEnabled` (`self.SplineMesh2`) (`self.Collision`))
          (`SceneComponent.K2_AttachToComponent` (`self.SplineMesh2`) null "None" "KeepRelative" "KeepRelative" "KeepRelative" true)
          (`SplineMeshComponent.SetStartAndEnd` (`self.SplineMesh2`) _location_6 (* _tangent_6 -1.0) _location_3 (* _tangent_3 -1.0) true))))))