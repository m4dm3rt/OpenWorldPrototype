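; Base projectile hit impact actor that plays particle and sound effects at a hit result's impact point.
; On BeginPlay it casts the hit actor to Pawn to choose between pawn and environment effect events.
; Each event has a default implementation that spawns its emitter and sound.
; The actor then destroys itself immediately unless a life span is set.
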(event `self.ReceiveBeginPlay`
  ;[1 0 0] trigget spawning impact effects
  (`self.SpawnImpactEffects`)
  (`self.TryToDestroyHitImpact`))

(event `TryToDestroyHitImpact`
  ;[1 0 0] Destroy self if life span wasn't set
  (if (<= (`self.GetLifeSpan`) 0.0)
    (`self.K2_DestroyActor`)))

(event `SpawnImpactEffects`
  ;[1 0 0] decide what was hit and trigger proper event
  (cast `Pawn` (`.HitActor` (`GameplayStatics.BreakHitResult` (`self.HitResult`)))
    (:`then`
      (`self.SpawnHitPawnEffects`))
    (:`CastFailed`
      (`self.SpawnHitEnvironmentEffects`))))

(event `SpawnHitPawnEffects`
  (bind (_bblockinghit _binitialoverlap _time _distance _location _impactpoint) (`GameplayStatics.BreakHitResult` (`self.HitResult`)))
  ;[1 0 0] Hit Pawn default implementation
  (`GameplayStatics.SpawnEmitterAtLocation` (`self.HitPawnVFX`) _impactpoint)
  (`GameplayStatics.SpawnSoundAtLocation` (`self.HitPawnSFX`) _impactpoint (struct) 1.0 1.0 0.0 null null))

(event `SpawnHitEnvironmentEffects`
  (bind (_bblockinghit _binitialoverlap _time _distance _location _impactpoint) (`GameplayStatics.BreakHitResult` (`self.HitResult`)))
  ;[1 0 0] Hit environment default implementation
  (`GameplayStatics.SpawnEmitterAtLocation` (`self.HitEnvironmentVFX`) _impactpoint)
  (`GameplayStatics.SpawnSoundAtLocation` (`self.HitEnvironmentSFX`) _impactpoint (struct) 1.0 1.0 0.0 null null))

(fn `UserConstructionScript`)