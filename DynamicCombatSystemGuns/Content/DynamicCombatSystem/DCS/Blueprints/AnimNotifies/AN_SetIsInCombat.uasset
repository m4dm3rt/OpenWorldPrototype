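; Anim notify in the Dynamic Combat System that switches the IsInCombat activity on the animated mesh's owner at a point in an animation.
; Depending on its EnableCombat flag, it adds the non-stacking activity to, or removes it from, the owner's BP_StateManagerComponent.
; The notify name shows the flag's value on the animation timeline.
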(fn `GetNotifyName`
  (returns (ReturnValue :type String))
  (return (`KismetStringLibrary.Concat_StrStr` "Is In Combat: " (`KismetStringLibrary.Conv_BoolToString` (`self.EnableCombat`)))))

(fn `Received_Notify`
  (params (MeshComp :type "SkeletalMeshComponent Object Reference") (Animation :type "AnimSequenceBase Object Reference") (EventReference :type "AnimNotifyEventReference Structure (by ref)"))
  (returns (ReturnValue :type Boolean))
  (bind _returnvalue (`ActorComponent.GetOwner` MeshComp))
  (bind _returnvalue_2 (`Actor.GetComponentByClass` _returnvalue "/Game/DynamicCombatSystem/DCS/Blueprints/Components/StateManager/BP_StateManagerComponent.BP_StateManagerComponent_C"))
  ;[1 0 0] Switch IsInCombat activity on owner
  (`/Engine/EditorBlueprintResources/StandardMacros.IsValid` _returnvalue
    (:`Is Valid`
      (if (`self.EnableCombat`)
        (`/Game/DynamicCombatSystem/DCS/Blueprints/Components/StateManager/BP_StateManagerComponent.AddActivity` _returnvalue_2 (struct :`TagName` "Activity.IsInCombat") false false)
        (else
          (`/Game/DynamicCombatSystem/DCS/Blueprints/Components/StateManager/BP_StateManagerComponent.RemoveActivity` _returnvalue_2 (struct :`TagName` "Activity.IsInCombat") false)))
      (return false))))