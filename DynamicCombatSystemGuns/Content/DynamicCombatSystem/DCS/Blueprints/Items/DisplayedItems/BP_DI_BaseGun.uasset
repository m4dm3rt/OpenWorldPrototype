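; BP_DI_BaseGun is the base displayed-item Blueprint for guns in the Dynamic Combat System.
; It plays montages, such as firing or reloading, on the GunMesh anim instance through an interface event.
; It returns the projectile spawn location from a GunMesh socket whose name comes from SocketsSolverObj.
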(event `/Game/DynamicCombatSystem/DCS/Blueprints/Interfaces/DisplayedItems/I_DisplayedItem_PlayMontage.PlayMontage`
  (params (Montage :type "AnimMontage Object Reference") (PlayRate :type "Float (double-precision)"))
  ;[1 0 0] Play anim montage - interface function
  ; used to play anims like fire gun / reload
  (`AnimInstance.Montage_Play` (`SkeletalMeshComponent.GetAnimInstance` (`self.GunMesh`)) Montage PlayRate "Duration" 0.0 true))

(fn `GetProjectileSpawnLocation`
  (returns (SpawnLocation :type "Vector Structure"))
  (return (`SceneComponent.GetSocketLocation` (`self.GunMesh`) (`/Game/DynamicCombatSystem/DCS/Blueprints/Items/DisplayedItems/AttachmentSolver/BP_BaseItemSocketsSolver.GetProjectileSpawnSocketName` (`self.SocketsSolverObj`)))))

(fn `UserConstructionScript`
  (`parent.UserConstructionScript`))