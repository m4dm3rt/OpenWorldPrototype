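; Bullet variant of a trace projectile in the guns module, which supplies the visual bullet trail for a shot.
; SpawnTracerEffect spawns the Niagara weapon-fire tracer at the actor's location and sets its trigger parameter.
; It feeds the trail's end to the system's impact-position array: the impact point on a blocking hit, otherwise the point at max range along the actor's forward vector.
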(fn `SpawnTracerEffect`
  (params (HitResult :type "HitResult Structure (by ref)"))
  (bind (_bblockinghit _binitialoverlap _time _distance _location _impactpoint) (`GameplayStatics.BreakHitResult` HitResult))
  ;[1 0 0] Play tracer effect ( bullet trail )
  (bind _returnvalue (`NiagaraFunctionLibrary.SpawnSystemAtLocation` "/Game/DynamicCombatSystem/GunsModule/VFX/Guns/Particles/Weapons/NS_WeaponFire_Tracer.NS_WeaponFire_Tracer" (`self.K2_GetActorLocation`) (`KismetMathLibrary.MakeRotator` 0.0 0.0 90.0)))
  (`NiagaraComponent.SetVariableBool` _returnvalue "User.Trigger" true)
  (`NiagaraDataInterfaceArrayFunctionLibrary.SetNiagaraArrayVector` _returnvalue "User.ImpactPositions" (`|MakeArray` (select `bool` _bblockinghit :`false` (+ (`self.K2_GetActorLocation`) (* (`self.GetActorForwardVector`) (`self.MaxRange`))) :`true` _impactpoint))))

(fn `UserConstructionScript`
  (`parent.UserConstructionScript`))