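; Actor component that registers itself as an indicator with the minimap UI.
; On BeginPlay it finds every W_MiniMapMaster widget, including nested ones, and calls AddIndicator with itself; EndPlay mirrors this with RemoveIndicator.
; Both paths are skipped on dedicated servers.
; Registration is a one-time search, so this component does not register with minimap widgets created after its BeginPlay.
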(event `self.ReceiveBeginPlay`
  (if (not (`KismetSystemLibrary.IsDedicatedServer`))
    (bind _foundwidgets (`WidgetBlueprintLibrary.GetAllWidgetsOfClass` "/Game/ModularInterfacePack/ModularMiniMapSystem/BP/Widgets/Master/W_MiniMapMaster.W_MiniMapMaster_C" false))
    (for _array_element _foundwidgets
      (`/Game/ModularInterfacePack/ModularMiniMapSystem/BP/Widgets/Master/W_MiniMapMaster.AddIndicator` _array_element self))))

(event `self.ReceiveEndPlay`
  (params (EndPlayReason :type "EEndPlayReason Enum" :default "Destroyed"))
  (if (not (`KismetSystemLibrary.IsDedicatedServer`))
    (bind _foundwidgets (`WidgetBlueprintLibrary.GetAllWidgetsOfClass` "/Game/ModularInterfacePack/ModularMiniMapSystem/BP/Widgets/Master/W_MiniMapMaster.W_MiniMapMaster_C" false))
    (for _array_element _foundwidgets
      (`/Game/ModularInterfacePack/ModularMiniMapSystem/BP/Widgets/Master/W_MiniMapMaster.RemoveIndicator` _array_element self))))